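; BP_Planet is a planet actor that builds its dynamic mesh at BeginPlay from one of several pre-made static meshes.
; A switch on Divs, currently forced to 4, selects the subdivision mesh to copy in through Geometry Script.
; On success it assigns land and ocean materials, prints a debug message, and passes the triangle polygroup IDs to CachePolygroupsByTriangle.
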(event `self.ReceiveBeginPlay`
  (bind _geometryscriptindexlist (make `GeometryScriptIndexList` "Any"))
  (set `self.divs` 4)
  (bind _returnvalue (`BaseDynamicMeshComponent.GetDynamicMesh` (`self.DynamicMeshComponent`)))
  (set `self.DynamicMesh` _returnvalue)
  (switch `int` (`self.divs`)
    (:`4`
      (`GeometryScriptLibrary_StaticMeshFunctions.CopyMeshFromStaticMesh` "/Game/div4.div4" _returnvalue (struct) (struct) null
        (:`Success`
          _)))
    (:`5`
      (`GeometryScriptLibrary_StaticMeshFunctions.CopyMeshFromStaticMesh` "/Game/div5.div5" _returnvalue (struct) (struct) null
        (:`Success`
          _)))
    (:`6`
      (`GeometryScriptLibrary_StaticMeshFunctions.CopyMeshFromStaticMesh` "/Game/div6.div6" _returnvalue (struct) (struct) null
        (:`Success`
          _)))
    (:`7`
      (`GeometryScriptLibrary_StaticMeshFunctions.CopyMeshFromStaticMesh` "/Game/div7.div7" _returnvalue (struct) (struct) null
        (:`Success`
          _)))
    (:`8`
      (`GeometryScriptLibrary_StaticMeshFunctions.CopyMeshFromStaticMesh` "/Game/div8.div8" _returnvalue (struct) (struct) null
        (:`Success`
          _))))
  (`PrimitiveComponent.SetMaterial` (`self.DynamicMeshComponent`) 0 "/Game/texturesAndMats/Land_Mat.Land_Mat")
  (`PrimitiveComponent.SetMaterial` (`self.DynamicMeshComponent`) 1 "/Game/texturesAndMats/Ocean_Mat.Ocean_Mat")
  (`KismetSystemLibrary.PrintString` "Mesh copied from static mesh" true true (struct :`R` 0.019812 :`G` 1.0 :`B` 0.04238 :`A` 1.0) 99.0)
  (`GeometryScriptLibrary_MeshPolygroupFunctions.GetAllTrianglePolygroupIDs` (`self.DynamicMesh`) (struct) _geometryscriptindexlist)
  (bind _indexarray (`GeometryScriptLibrary_ListUtilityFunctions.ConvertIndexListToArray` _geometryscriptindexlist))
  (`self.CachePolygroupsByTriangle` _indexarray))

(fn `UserConstructionScript`)