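; BP_Person is a clickable unit Blueprint representing a person owned by a player on what appears to be a globe map.
; Clicking its Quinn skeletal mesh on a client without authority passes the unit to the local BP_GlobePlayerController through OnUnitClickCallback.
; GetTitle returns a display string naming the unit type and the owning player's ID.
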(event `self.SKM_Quinn.OnClicked`
  (params (TouchedComponent :type "PrimitiveComponent Object Reference") (ButtonPressed :type "Key Structure"))
  (`/Engine/EditorBlueprintResources/ActorMacros.Switch Has Authority`
    (:`Remote`
      (bind _asbp_globe_player_controller (cast `/Game/BP_GlobePlayerController` (`GameplayStatics.GetPlayerController` 0)))
      (`/Game/BP_GlobePlayerController.OnUnitClickCallback` _asbp_globe_player_controller self))))

(event `self.ReceiveBeginPlay`)

(fn `Get Title`
  (returns (`Unit Title` :type String))
  (return (`KismetStringLibrary.Concat_StrStr` (`KismetStringLibrary.Concat_StrStr` "Unit: Person\\n" "Owned by player ") (`KismetStringLibrary.Conv_IntToString` (`self.OwningPlayerID`)))))

(fn `UserConstructionScript`)