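; Procedural globe actor that builds a clickable land-and-ocean world from a dynamic mesh, with each face as a polygroup.
; Tick adds faces in batches adapted to frame time, then builds collision, reveals the mesh and signals load completion.
; Remote clicks resolve triangles to face IDs for the player controller.
; Server events spawn owned units on faces and relay recoloring through a multicast that caches one dynamic material per color.
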(event `Color Face By Triangle ID SERVER`
  (params (`Triangle ID` :type Integer) (Color :type "LinearColor Structure"))
  (bind _returnvalue (`self.Triangle ID to Face ID` `Triangle ID`))
  (`self.Color Face By Face ID MULTI` _returnvalue Color))

(event `Color Face By Face ID SERVER`
  (params (`Triangle ID` :type Integer) (Color :type "LinearColor Structure"))
  (`self.Color Face By Face ID MULTI` `Triangle ID` Color))

(event `Color Face By Face ID MULTI`
  (params (`Face ID` :type Integer) (Color :type "LinearColor Structure"))
  (bind _geometryscriptindexlist (make `GeometryScriptIndexList` "Triangle"))
  (bind _returnvalue (`PrimitiveComponent.GetNumMaterials` (`self.DynamicMesh`)))
  (if (not (`BlueprintMapLibrary.Map_Contains` (`self.colorToMaterialIndexMap`) Color))
    ;[1 1 1] Create new Dynamic Material Instance and add it to colorToMaterialIndex
    (bind _returnvalue_2 (`PrimitiveComponent.CreateDynamicMaterialInstance` (`self.DynamicMesh`) _returnvalue "/Game/texturesAndMats/SetColorMat_Inst.SetColorMat_Inst" "None"))
    (`MaterialInstanceDynamic.SetVectorParameterValue` _returnvalue_2 "Color" Color)
    (`BlueprintMapLibrary.Map_Add` (`self.colorToMaterialIndexMap`) Color (- _returnvalue 1)))
  ;[1 1 1] Get DynamicMaterialInstance from map, and set the material on the face
  (bind _returnvalue_3 (`GeometryScriptLibrary_MeshPolygroupFunctions.GetTrianglesInPolygroup` (`self.unwrappedDynamicMesh`) (struct) `Face ID` _geometryscriptindexlist))
  (`GeometryScriptLibrary_MeshMaterialFunctions.SetMaterialIDOnTriangles` _returnvalue_3 _geometryscriptindexlist (`BlueprintMapLibrary.Map_Find` (`self.colorToMaterialIndexMap`) Color) false null))

(event `self.ReceiveBeginPlay`
  (bind _dynamicmesh (`self.DynamicMesh`))
  ;[1 1 1 0.2] Load the world
  (`self.GenerateWorld` 4)
  (bind _returnvalue (`BaseDynamicMeshComponent.GetDynamicMesh` (`self.DynamicMesh`)))
  (set `self.unwrappedDynamicMesh` _returnvalue)
  (`PrimitiveComponent.SetMaterial` _dynamicmesh 0 "/Game/texturesAndMats/Land_Mat.Land_Mat")
  (`PrimitiveComponent.SetMaterial` _dynamicmesh 1 "/Game/texturesAndMats/Ocean_Mat.Ocean_Mat")
  (bind _returnvalue_2 (`self.GetAllVerticeLocations`))
  (bind _vectorlist (`GeometryScriptLibrary_ListUtilityFunctions.ConvertArrayToVectorList` _returnvalue_2))
  (`GeometryScriptLibrary_MeshBasicEditFunctions.AddVerticesToMesh` (`self.unwrappedDynamicMesh`) _vectorlist)
  (bind _returnvalue_3 (`self.GetFaceCount`))
  (set `self.GlobeFaces` _returnvalue_3)
  (`SceneComponent.SetHiddenInGame` (`self.DynamicMesh`) true false))

(event `Spawn Person At Face SERVER`
  (params (playerController :type "/Game/BP_GlobePlayerController Object Reference") (`Face Id` :type Integer))
  (bind _returnvalue (`self.GetMidpointOfFace` `Face Id`))
  (bind _returnvalue_2 (`|SpawnActorFromClass` "/Game/BP_Person.BP_Person_C" (`KismetMathLibrary.MakeTransform` _returnvalue (`KismetMathLibrary.MakeRotFromZ` _returnvalue)) "Undefined" "MultiplyWithRoot" null null))
  (set `/Game/BP_Person.OwningPlayerID` (`/Game/BP_GlobePlayerController.playerId` playerController) _returnvalue_2)
  (set `/Game/BP_Person.Face Id` `Face Id` _returnvalue_2)
  (set `/Game/BP_Person.playerController` playerController _returnvalue_2)
  (`KismetArrayLibrary.Array_Add` (`/Game/BP_GlobePlayerController.units` playerController) _returnvalue_2)
  (bind _returnvalue_3 (`GameplayStatics.GetActorOfClass` "/Game/GlobeGameMode.GlobeGameMode_C"))
  (`/Game/GlobeGameMode.OnUnitSpawned` _returnvalue_3 _returnvalue_2))

(event `self.ReceiveTick`
  (params (DeltaSeconds :type "Float (single-precision)"))
  (bind _facestospawnperframe (`self.facesToSpawnPerFrame`))
  (bind _spawnedfaces (`self.spawnedFaces`))
  (bind _dynamicmesh (`self.DynamicMesh`))
  (if (> DeltaSeconds 0.2)
    (`/Engine/EditorBlueprintResources/StandardMacros.DecrementInt` _facestospawnperframe
      (:`  `
        _))
    (else
      (`/Engine/EditorBlueprintResources/StandardMacros.IncrementInt` _facestospawnperframe
        (:`  `
          _))))
  (for _ (range (+ (`KismetMathLibrary.Max` (`self.facesToSpawnPerFrame`)) 1))
    (if (< (`self.spawnedFaces`) (`self.GlobeFaces`))
      (bind _returnvalue (`self.GetTriangleIntVectorsForFaceByIndex` _spawnedfaces))
      (bind _trianglelist (`GeometryScriptLibrary_ListUtilityFunctions.ConvertArrayToTriangleList` _returnvalue))
      (bind _newindiceslist (`GeometryScriptLibrary_MeshBasicEditFunctions.AddTrianglesToMesh` (`self.unwrappedDynamicMesh`) _trianglelist _spawnedfaces false null))
      (bind _returnvalue_2 (`self.isFaceWater` (`self.spawnedFaces`)))
      (if _returnvalue_2
        (`GeometryScriptLibrary_MeshMaterialFunctions.SetMaterialIDOnTriangles` (`self.unwrappedDynamicMesh`) _newindiceslist 1 false null))
      (`/Engine/EditorBlueprintResources/StandardMacros.IncrementInt` (`self.spawnedFaces`))
      (else
        (bind _output_get (set `self.isDoneSpawningFaces` true))
        (break))))
  (if _output_get
    (`self.SetActorTickEnabled` false)
    (bind _returnvalue_3 (`BaseDynamicMeshComponent.GetDynamicMesh` _dynamicmesh))
    (`GeometryScriptLibrary_CollisionFunctions.SetDynamicMeshCollisionFromMesh` _returnvalue_3 _dynamicmesh (struct) null)
    (`SceneComponent.SetHiddenInGame` _dynamicmesh false false)
    (`self.OnGlobeLoadComplete`)))

(event `self.DynamicMesh.OnClicked`
  (params (TouchedComponent :type "PrimitiveComponent Object Reference") (ButtonPressed :type "Key Structure"))
  (`/Engine/EditorBlueprintResources/ActorMacros.Switch Has Authority`
    (:`Remote`
      (bind _asbp_globe_player_controller (cast `/Game/BP_GlobePlayerController` (`GameplayStatics.GetPlayerController` 0)))
      (bind (_hitresult _returnvalue) (`PlayerController.GetHitResultUnderCursorByChannel` _asbp_globe_player_controller "TraceTypeQuery2" true))
      (if _returnvalue
        (bind (_outhit _returnvalue_2) (`KismetSystemLibrary.LineTraceSingle` (* (`.ImpactPoint` (`GameplayStatics.BreakHitResult` _hitresult)) 1.01) (0.0 0.0 0.0) "TraceTypeQuery2" true (`|MakeArray` (`Controller.K2_GetPawn` _asbp_globe_player_controller) :!type "Actor Object Reference") "Persistent" false))
        (if _returnvalue_2
          (bind _returnvalue_3 (`self.Triangle ID to Face ID` (`.FaceIndex` (`GameplayStatics.BreakHitResult` _outhit))))
          (`/Game/BP_GlobePlayerController.OnGlobeClickCallback` _asbp_globe_player_controller TouchedComponent ButtonPressed _returnvalue_3))))))

(fn `Get Initial Spawnable Tile ID`
  (returns (faceId :type Integer))
  (locals (SpawnableTileID :type Integer))
  (set `local.SpawnableTileID` -1)
  (while (== (`local.SpawnableTileID`) -1)
    (set `local.SpawnableTileID` (`KismetMathLibrary.RandomInteger` (`self.GlobeFaces`)))
    (bind _returnvalue (`self.isFaceWater` (`local.SpawnableTileID`)))
    (if _returnvalue
      (set `local.SpawnableTileID` -1)))
  (return (`local.SpawnableTileID`)))

(fn `Triangle ID to Face ID`
  (params (TriangleID :type Integer))
  (returns (ReturnValue :type Integer))
  (return (`.ReturnValue` (`GeometryScriptLibrary_MeshPolygroupFunctions.GetTrianglePolygroupID` (`self.unwrappedDynamicMesh`) (struct) TriangleID))))

(fn `UserConstructionScript`)