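; AI controller for a globe turn-based game that plays a BP_GlobePlayerPawn with random moves.
; It caches the possessed pawn, and GetNextMove returns a random move from that pawn's first unmoved unit, resolved by UUID through BP_GlobeGameMode.
; An empty move or no unmoved units sets WaitingOnTurn on the pawn's private player state.
; The game mode's pass-turn event clears that flag.
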(event `self.ReceiveBeginPlay`
  (bind _returnvalue (`GameplayStatics.GetActorOfClass` "/Game/BP_GlobeGameMode.BP_GlobeGameMode_C"))
  (bind _output_get (set `self.gameMode` _returnvalue))
  (add `/Game/BP_GlobeGameMode.PassTurn` _output_get (delegate `OnTurnPassed`)))

(event `OnTurnPassed`
  (set `/Game/BP_PrivatePlayerState.waitingOnTurn` false (`/Game/BP_GlobePlayerPawn.privatePlayerState` (`self.globePlayerPawn`))))

(event `self.ReceivePossess`
  (params (PossessedPawn :type "Pawn Object Reference"))
  (bind _asbp_globe_player_pawn (cast `/Game/BP_GlobePlayerPawn` PossessedPawn)
    (:`then`
      (set `self.globePlayerPawn` _asbp_globe_player_pawn))
    (:`CastFailed`
      (`KismetSystemLibrary.PrintString` "AI rand: onpossess cast failed"))))

(fn `GetNextMove`
  (returns (`Next Move` :type "/Game/BP_UnitMove Object Reference"))
  (for _array_element (`/Game/BP_GlobePlayerPawn.unitReferencesForControllerUse` (`self.globePlayerPawn`))
    (bind _unit (`/Game/BP_GlobeGameMode.Get Unit by UUID` (`self.gameMode`) (`.UUID_3_947EECCF4DC50D5EA07702BE29C743A4` (break `/Game/BP_Struct_Unit_Reference` _array_element))))
    (if (not (`/Game/BP_Person.hasMoved` _unit))
      (bind _outputmove (`/Game/BP_Person.GetRandomMove` _unit))
      (if (== _outputmove null)
        (set `/Game/BP_PrivatePlayerState.waitingOnTurn` true (`/Game/BP_GlobePlayerPawn.privatePlayerState` (`self.globePlayerPawn`)) :!label _label)
        (return null)
        (else
          (return _outputmove)))))
  (goto _label))

(fn `OnRep_IsEnabled`
  (if (`self.IsEnabled`)
    _))

(fn `Set Actor References`)

(fn `UserConstructionScript`)