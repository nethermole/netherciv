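; Game mode for the multiplayer lobby, holding the lobby info struct and giving the lobby a short random GUID-based name.
; On login it assigns each player a client ID, records their name in the game instance and makes the first player owner.
; Joins and setting changes rebuild the struct from player controllers and push it manually to the game state.
; Starting finalizes info through each controller, then server-travels to the procedural globe after a delay.
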(event `self.ReceiveBeginPlay`
  (bind (_playernames _lobbyowner _subdivisions _numhumans _numbots _mapgenerationtype) (break `/Game/MultiplayerLobby/Struct_ClientLobbyInfo` (`self.Lobby Info`)))
  (bind _output_get (set `self.Lobby Info` (make `/Game/MultiplayerLobby/Struct_ClientLobbyInfo` _playernames _lobbyowner _subdivisions _numhumans _numbots _mapgenerationtype (`KismetStringLibrary.GetSubstring` (`KismetGuidLibrary.Conv_GuidToString` (`KismetGuidLibrary.NewGuid`)) 0 5))))
  (`/Game/BP_FL_Logging.Log` (`KismetStringLibrary.Concat_StrStr` "Server opened with name: " (`.LobbyName_22_C5D107594FE50181DFBA4DB4DBFF6D06` (break `/Game/MultiplayerLobby/Struct_ClientLobbyInfo` _output_get)) "\""))
  (`/Game/BP_FL_Logging.Log` "End beginplay"))

(event `Update Lobby Info To Players`
  (bind _lobby_info (`self.Manually Replicate Lobby Info to Player Controllers`))
  (bind _outactors (`GameplayStatics.GetAllActorsOfClass` "/Game/MultiplayerLobby/BP_GameStateBase_MultiplayerLobby.BP_GameStateBase_MultiplayerLobby_C"))
  (for _array_element _outactors
    (`/Game/MultiplayerLobby/BP_GameStateBase_MultiplayerLobby.Update Lobby Info` _array_element _lobby_info)))

(event `StartGamePressed`
  (bind _outactors (`GameplayStatics.GetAllActorsOfClass` "/Game/MultiplayerLobby/BP_PlayerController_MultiplayerLobby.BP_PlayerController_MultiplayerLobby_C"))
  (for _array_element _outactors
    (`/Game/MultiplayerLobby/BP_PlayerController_MultiplayerLobby.Finalize Lobby Info to GameInstance` _array_element (`self.Lobby Info`)))
  (`KismetSystemLibrary.Delay` 1.0)
  (`KismetSystemLibrary.ExecuteConsoleCommand` "ServerTravel BP_L_ProceduralGlobe" null))

(event `self.K2_PostLogin`
  (params (NewPlayer :type "PlayerController Object Reference"))
  (bind _asbp_player_controller_multiplayer_lobby (cast `/Game/MultiplayerLobby/BP_PlayerController_MultiplayerLobby` NewPlayer))
  (`/Game/BP_FL_Logging.Log` (`KismetStringLibrary.Concat_StrStr` "Event OnPostLogin called. Current lobby name is " (`.LobbyName_22_C5D107594FE50181DFBA4DB4DBFF6D06` (break `/Game/MultiplayerLobby/Struct_ClientLobbyInfo` (`self.Lobby Info`)))))
  (bind _player_name (`/Game/MultiplayerLobby/BP_PlayerController_MultiplayerLobby.Player Name` _asbp_player_controller_multiplayer_lobby))
  (`/Game/BP_FL_Logging.Log` (`KismetStringLibrary.Concat_StrStr` "New Player: \"" "" _player_name))
  (`/Game/MultiplayerLobby/BP_PlayerController_MultiplayerLobby.LogStringSentFromServer` _asbp_player_controller_multiplayer_lobby (`KismetStringLibrary.Concat_StrStr` "Successfully connected to server \"" (`.LobbyName_22_C5D107594FE50181DFBA4DB4DBFF6D06` (break `/Game/MultiplayerLobby/Struct_ClientLobbyInfo` (`self.Lobby Info`))) "\""))
  (bind _asbp_game_instance (cast `/Game/Multiplayer/BP_GameInstance` (`GameplayStatics.GetGameInstance`)))
  (bind _output_get (set `/Game/MultiplayerLobby/BP_PlayerController_MultiplayerLobby.Assigned Client ID` (`KismetGuidLibrary.Conv_GuidToString` (`KismetGuidLibrary.NewGuid`)) _asbp_player_controller_multiplayer_lobby))
  (`/Game/Multiplayer/BP_GameInstance.Add Player Name By Assigned Id` _asbp_game_instance _output_get _player_name)
  ;[1 1 1] Check whether to set controller as lobby owner
  (if (== (`self.Lobby Owner`) null)
    (set `self.Lobby Owner` _asbp_player_controller_multiplayer_lobby))
  (`self.Update Lobby Info To Players`))

(event `Update Subdivisions`
  (params (Subdivisions :type Integer))
  (bind _structout (setmembers `/Game/MultiplayerLobby/Struct_ClientLobbyInfo` :`StructRef` (`self.Lobby Info`)))
  (set `self.Lobby Info` (make `/Game/MultiplayerLobby/Struct_ClientLobbyInfo` (break `/Game/MultiplayerLobby/Struct_ClientLobbyInfo` _structout) (`.LobbyOwner_7_537E05C0440C57C0785F63B99AACF196` (break `/Game/MultiplayerLobby/Struct_ClientLobbyInfo` _structout)) Subdivisions (`.NumHumans_15_4B5DEA2449C45E5DF568E695F664193A` (break `/Game/MultiplayerLobby/Struct_ClientLobbyInfo` _structout)) (`.NumBots_16_D4C4C9364EF343C21233CEAD1B2ED9C2` (break `/Game/MultiplayerLobby/Struct_ClientLobbyInfo` _structout)) (`.MapGenerationType_19_DE8196274DD9D74D09095A9CF8260891` (break `/Game/MultiplayerLobby/Struct_ClientLobbyInfo` _structout)) (`.LobbyName_22_C5D107594FE50181DFBA4DB4DBFF6D06` (break `/Game/MultiplayerLobby/Struct_ClientLobbyInfo` _structout))))
  (`self.Update Lobby Info To Players` :!label _label))

(event `Update Num Bots`
  (params (`Num Bots` :type Integer))
  (bind _structout (setmembers `/Game/MultiplayerLobby/Struct_ClientLobbyInfo` :`StructRef` (`self.Lobby Info`)))
  (set `self.Lobby Info` (make `/Game/MultiplayerLobby/Struct_ClientLobbyInfo` (break `/Game/MultiplayerLobby/Struct_ClientLobbyInfo` _structout) (`.LobbyOwner_7_537E05C0440C57C0785F63B99AACF196` (break `/Game/MultiplayerLobby/Struct_ClientLobbyInfo` _structout)) (`.Subdivisions_14_E843781C4EEE8E83DA68248EA9C359BE` (break `/Game/MultiplayerLobby/Struct_ClientLobbyInfo` _structout)) (`.NumHumans_15_4B5DEA2449C45E5DF568E695F664193A` (break `/Game/MultiplayerLobby/Struct_ClientLobbyInfo` _structout)) `Num Bots` (`.MapGenerationType_19_DE8196274DD9D74D09095A9CF8260891` (break `/Game/MultiplayerLobby/Struct_ClientLobbyInfo` _structout)) (`.LobbyName_22_C5D107594FE50181DFBA4DB4DBFF6D06` (break `/Game/MultiplayerLobby/Struct_ClientLobbyInfo` _structout))))
  (goto _label))

(fn `Manually Replicate Lobby Info to Player Controllers`
  (returns (`Lobby Info` :type "/Game/MultiplayerLobby/Struct_ClientLobbyInfo Structure"))
  (locals (`Player Names` :type "Array of String"))
  (bind _outactors (`GameplayStatics.GetAllActorsOfClass` "/Game/MultiplayerLobby/BP_PlayerController_MultiplayerLobby.BP_PlayerController_MultiplayerLobby_C"))
  (for _array_element _outactors
    (`KismetArrayLibrary.Array_Add` (`local.Player Names`) (`/Game/MultiplayerLobby/BP_PlayerController_MultiplayerLobby.Player Name` _array_element)))
  (bind _structout (setmembers `/Game/MultiplayerLobby/Struct_ClientLobbyInfo` :`StructRef` (`self.Lobby Info`)))
  (bind _output_get (set `self.Lobby Info` (make `/Game/MultiplayerLobby/Struct_ClientLobbyInfo` (`local.Player Names`) (`/Game/MultiplayerLobby/BP_PlayerController_MultiplayerLobby.Player Name` (`self.Lobby Owner`)) (`.Subdivisions_14_E843781C4EEE8E83DA68248EA9C359BE` (break `/Game/MultiplayerLobby/Struct_ClientLobbyInfo` _structout)) (`GameplayStatics.GetNumPlayerControllers`) (`.NumBots_16_D4C4C9364EF343C21233CEAD1B2ED9C2` (break `/Game/MultiplayerLobby/Struct_ClientLobbyInfo` _structout)) (`.MapGenerationType_19_DE8196274DD9D74D09095A9CF8260891` (break `/Game/MultiplayerLobby/Struct_ClientLobbyInfo` _structout)) (`.LobbyName_22_C5D107594FE50181DFBA4DB4DBFF6D06` (break `/Game/MultiplayerLobby/Struct_ClientLobbyInfo` _structout)))))
  (return _output_get))

(fn `UserConstructionScript`)