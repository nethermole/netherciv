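; Player controller for the multiplayer lobby that creates the lobby widget for the local player and relays lobby actions.
; Start-game and setting changes (subdivisions, human and bot counts) are forwarded to the lobby GameMode.
; Current lobby info is read from the lobby GameState, and a finalize event copies the LobbyInfo it receives into the GameInstance.
; A further event logs text sent from the server.
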(event `self.ReceiveBeginPlay`
  (if (`self.IsLocalPlayerController`)
    (bind _returnvalue (`|CreateWidget` "/Game/MultiplayerLobby/UI/WB_MultiplayerLobby.WB_MultiplayerLobby_C" self))
    (`UserWidget.AddToViewport` _returnvalue 0)))

(event `Start Game Pressed`
  (bind _asbp_gm_multiplayer_lobby (cast `/Game/MultiplayerLobby/BP_GM_MultiplayerLobby` (`GameplayStatics.GetGameMode`)))
  (`/Game/MultiplayerLobby/BP_GM_MultiplayerLobby.StartGamePressed` _asbp_gm_multiplayer_lobby))

(event `Finalize Lobby Info to GameInstance`
  (params (`Lobby Info` :type "/Game/MultiplayerLobby/Struct_ClientLobbyInfo Structure"))
  (bind _asbp_game_instance (cast `/Game/Multiplayer/BP_GameInstance` (`GameplayStatics.GetGameInstance`)))
  (set `/Game/Multiplayer/BP_GameInstance.Lobby Info` `Lobby Info` _asbp_game_instance))

(event `LogStringSentFromServer`
  (params (Text :type String))
  (`/Game/BP_FL_Logging.Log` Text))

(event `Update Subdivisions`
  (params (Subdivisions :type Integer))
  (bind _asbp_gm_multiplayer_lobby (cast `/Game/MultiplayerLobby/BP_GM_MultiplayerLobby` (`GameplayStatics.GetGameMode`)))
  (`/Game/MultiplayerLobby/BP_GM_MultiplayerLobby.Update Subdivisions` _asbp_gm_multiplayer_lobby Subdivisions))

(event `Update Num Humans`
  (params (`Num Humans` :type Integer))
  (bind _asbp_gm_multiplayer_lobby (cast `/Game/MultiplayerLobby/BP_GM_MultiplayerLobby` (`GameplayStatics.GetGameMode`)))
  (`/Game/MultiplayerLobby/BP_GM_MultiplayerLobby.Update Num Humans` _asbp_gm_multiplayer_lobby `Num Humans`))

(event `Update Num Bots`
  (params (`Num Bots` :type Integer))
  (bind _asbp_gm_multiplayer_lobby (cast `/Game/MultiplayerLobby/BP_GM_MultiplayerLobby` (`GameplayStatics.GetGameMode`)))
  (`/Game/MultiplayerLobby/BP_GM_MultiplayerLobby.Update Num Bots` _asbp_gm_multiplayer_lobby `Num Bots`))

(fn `Get Lobby Info`
  (returns (`Lobby Info` :type "/Game/MultiplayerLobby/Struct_ClientLobbyInfo Structure"))
  (bind _asbp_game_state_base_multiplayer_lobby (cast `/Game/MultiplayerLobby/BP_GameStateBase_MultiplayerLobby` (`GameplayStatics.GetGameState`)))
  (return (`/Game/MultiplayerLobby/BP_GameStateBase_MultiplayerLobby.Lobby Info` _asbp_game_state_base_multiplayer_lobby)))

(fn `UserConstructionScript`)