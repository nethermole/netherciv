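; BP_GlobePlayerPawn is the player pawn for a globe-based game, handling actor lookup and player ID assignment.
; On BeginPlay it caches references to the BP_ProceduralGlobe and BP_GlobeGameState actors through GetActorOfClass.
; With authority only, it then takes an unset PlayerId from the game state's NextPlayerId counter, increments that counter and prints a debug message.
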(event `self.ReceiveBeginPlay`
  (`self.Set Actor References`)
  (`/Engine/EditorBlueprintResources/ActorMacros.Switch Has Authority`
    (:`Authority`
      (`self.Set Player Id`))))

(fn `Set Actor References`
  (bind _returnvalue (`GameplayStatics.GetActorOfClass` "/Game/BP_ProceduralGlobe.BP_ProceduralGlobe_C"))
  (set `self.proceduralGlobe` _returnvalue)
  (bind _returnvalue_2 (`GameplayStatics.GetActorOfClass` "/Game/BP_GlobeGameState.BP_GlobeGameState_C"))
  (set `self.gameState` _returnvalue_2))

(fn `Set Player Id`
  (bind _nextplayerid (`/Game/BP_GlobeGameState.nextPlayerId` (`self.gameState`)))
  (`/Engine/EditorBlueprintResources/ActorMacros.Switch Has Authority`
    (:`Authority`
      (if (== (`self.playerId`) -1)
        (`KismetSystemLibrary.PrintString` (`KismetStringLibrary.Concat_StrStr` "Id given to player " (`KismetStringLibrary.Conv_IntToString` _nextplayerid)) true true (struct :`G` 0.66 :`B` 1.0 :`A` 1.0) 100.0)
        (set `self.playerId` _nextplayerid)
        (`/Engine/EditorBlueprintResources/StandardMacros.IncrementInt` _nextplayerid)))))

(fn `UserConstructionScript`)