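; Blueprint array function library with a function that splits a struct-wrapped integer array into multiple such arrays based on a Size.
; It creates length / Size + 1 buckets in a map, then files each element by its value modulo that count.
; The buckets return as an array in index order.
; Grouping follows values rather than positions, so buckets can be uneven, empty or larger than Size.
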(fn `Break Struct Array Of Integer Into Multiple Array Of Integer Of Size`
  (params (Array :type "/Game/Struct_ArrayOfInteger Structure") (Size :type Integer :default 0))
  (returns (`Arrays Out` :type "Array of /Game/Struct_ArrayOfInteger Structure"))
  (locals (`Modulus buckets` :type "Map of Integer to /Game/Struct_ArrayOfInteger Structure") (`Modulus Bucket` :type "Array of /Game/Struct_ArrayOfInteger Structure") (bucketRef :type "Array of Integer"))
  (bind _intarray (break `/Game/Struct_ArrayOfInteger` Array))
  (bind _returnvalue (/ (`KismetArrayLibrary.Array_Length` _intarray) Size))
  (for _index (range (+ _returnvalue 1))
    (`BlueprintMapLibrary.Map_Add` (`local.Modulus buckets`) _index (make `/Game/Struct_ArrayOfInteger` _)))
  (for _array_element _intarray
    (bind _returnvalue_2 (mod _array_element (+ _returnvalue 1)))
    (bind _value (`BlueprintMapLibrary.Map_Find` (`local.Modulus buckets`) _returnvalue_2))
    (bind _output_get (set `local.bucketRef` (`.IntArray_4_E39F009D45F1E09EACD41D9D56F40223` (break `/Game/Struct_ArrayOfInteger` _value))))
    (`KismetArrayLibrary.Array_Add` _output_get _array_element)
    (bind _structout (setmembers `/Game/Struct_ArrayOfInteger` :`StructRef` _value :`IntArray` (`local.bucketRef`)))
    (`BlueprintMapLibrary.Map_Add` (`local.Modulus buckets`) _returnvalue_2 _structout))
  (for _index_2 (range (+ _returnvalue 1))
    (`KismetArrayLibrary.Array_Add` (`local.Modulus Bucket`) (`BlueprintMapLibrary.Map_Find` (`local.Modulus buckets`) _index_2)))
  (return (`local.Modulus Bucket`)))